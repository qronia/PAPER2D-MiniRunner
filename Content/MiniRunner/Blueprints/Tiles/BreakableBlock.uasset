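; BreakableBlock is a MiniRunner tile that breaks when a MovableBlock falls onto it.
; The construction script stops its flipbook on the first frame with looping off.
; On overlap with a MovableBlock moving downward fast enough, it plays the flipbook once and sets its lifespan to the flipbook length, so it is destroyed as the animation ends.
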(event `self.ReceiveActorBeginOverlap`
  (params (OtherActor :type "Actor Object Reference"))
  (bind _rendercomponent (`self.RenderComponent`))
  (bind _asmovable_block (cast `/Game/MiniRunner/Blueprints/Tiles/MovableBlock` OtherActor))
  (bind (_returnvalue_x _returnvalue_y _returnvalue_z) (`KismetMathLibrary.BreakVector` (`self.GetVelocity` _asmovable_block)))
  (if (<= _returnvalue_z -20.0)
    (`self.SetLifeSpan` (`PaperFlipbookComponent.GetFlipbookLength` _rendercomponent))
    (`PaperFlipbookComponent.PlayFromStart` _rendercomponent)))

(fn `UserConstructionScript`
  (bind _rendercomponent (`self.RenderComponent`))
  (`PaperFlipbookComponent.Stop` _rendercomponent)
  (`PaperFlipbookComponent.SetLooping` _rendercomponent false)
  (`PaperFlipbookComponent.SetNewTime` _rendercomponent 0.0))